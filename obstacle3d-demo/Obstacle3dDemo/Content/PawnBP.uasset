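; PawnBP is a camera pawn that orbits and zooms around its spring arm origin using the mouse.
; Each Tick adds vertical and horizontal mouse input to the SpringArm's relative pitch and yaw, and subtracts wheel input from its arm length.
; Both are scaled by sensitivity variables and frame delta time, with no clamping on pitch or zoom distance.
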(event `self.ReceiveTick`
  (params (DeltaSeconds :type "Float (single-precision)"))
  (bind _springarm (`self.SpringArm`))
  (bind _returnvalue (* (`self.RotationSensitivity`) (`GameplayStatics.GetWorldDeltaSeconds`)))
  (`SceneComponent.K2_AddRelativeRotation` _springarm (`KismetMathLibrary.MakeRotator` 0.0 (* (`self.GetInputAxisValue`) _returnvalue) (* _returnvalue (`self.GetInputAxisValue`))) false false)
  (set `SpringArmComponent.TargetArmLength` (- (`SpringArmComponent.TargetArmLength` _springarm) (* (`self.GetInputAxisValue`) (* (`self.ZoomSensitivity`) (`GameplayStatics.GetWorldDeltaSeconds`)))) _springarm))

(fn `UserConstructionScript`)